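; BP_PaperPlayer is a player Blueprint that controls the flash and opacity of its sprite through material parameters.
; On BeginPlay it creates a dynamic material instance from the Sprite's first material slot and stores it.
; SetSpriteFlash writes a flash multiplier and colour to that instance, and SetSpriteOpacity writes an opacity multiplier, so both effects act on the sprite at runtime.
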(event EventBeginPlay
  (bind _returnvalue (Rendering|Material|CreateDynamicMaterialInstance (Variables|Default|GetSprite) 0 0 "None" :!class /Script/Engine.PrimitiveComponent))
  (Variables|Default|SetMaterialInstance _returnvalue))

(event EventSetSpriteFlash
  (params (FlashMultiplier :type Float%20%28single-precision%29) (Colour :type Linear%20Color%20Structure))
  (Rendering|Material|SetScalarParameterValue (Variables|Default|GetMaterialInstance) "FlashMultiplier" FlashMultiplier :!class /Script/Engine.MaterialInstanceDynamic)
  (Rendering|Material|SetVectorParameterValue (Variables|Default|GetMaterialInstance) "FlashColour" Colour :!class /Script/Engine.MaterialInstanceDynamic))

(event EventSetSpriteOpacity
  (params (Opacity :type Float%20%28single-precision%29))
  (Rendering|Material|SetScalarParameterValue (Variables|Default|GetMaterialInstance) "OpacityMultiplier" Opacity :!class /Script/Engine.MaterialInstanceDynamic))

(fn ConstructionScript)